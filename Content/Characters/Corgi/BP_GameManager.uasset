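; BP_GameManager coordinates the corgi training game, linking stage progression, the dog's training component and the HUD.
; On BeginPlay it creates the HUD, finds the first BP_Corgi, binds its events and starts TrainingProgress at the Sit stage.
; Completed levels advance TrainingProgress, whose stage changes start the matching level on the dog's DogTraining.
; A looping timer pushes stage, cue, proficiency, unlocks and click-window state to the HUD instead of using Tick.
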(event `self.ReceiveBeginPlay`
  (`KismetSystemLibrary.K2_SetTimerDelegate` (delegate `RefreshHUD`) 0.1 true)
  (bind _returnvalue (`|CreateWidget` "/Game/Characters/Corgi/WBP_HUD.WBP_HUD_C"))
  (bind _output_get (set `self.HUDRef` _returnvalue))
  (`UserWidget.AddToViewport` _output_get 0)
  (bind _outactors (`GameplayStatics.GetAllActorsOfClass` "/Game/Characters/Corgi/BP_Corgi.BP_Corgi_C"))
  (set `self.DogRef` (`|GetArrayItem` _outactors))
  (add `DogTrainingComponent.OnLevelCompleted` (`/Game/Characters/Corgi/BP_Corgi.DogTraining` (`self.DogRef`)) (delegate `HandleLevelCompleted`))
  (add `TrainingProgressComponent.OnStageChanged` (`self.TrainingProgress`) (delegate `HandleLevelChange`))
  (`TrainingProgressComponent.InitializeProgress` (`self.TrainingProgress`))
  (`TrainingProgressComponent.StartStage` (`self.TrainingProgress`) "Sit"))

(event `HandleLevelCompleted`
  (params (CompletedStage :type "ECueType Enum" :default "None"))
  (`TrainingProgressComponent.AdvanceStage` (`self.TrainingProgress`)))

(event `HandleLevelChange`
  (params (NewStage :type "ECueType Enum" :default "None"))
  (`DogTrainingComponent.StartLevel` (`/Game/Characters/Corgi/BP_Corgi.DogTraining` (`self.DogRef`)) NewStage))

(event `RefreshHUD`
  (bind _trainingprogress (`self.TrainingProgress`))
  (bind _dogtraining (`/Game/Characters/Corgi/BP_Corgi.DogTraining` (`self.DogRef`)))
  (`/Game/Characters/Corgi/WBP_HUD.UpdateHUD` (`self.HUDRef`) (`TrainingProgressComponent.GetCurrentStage` _trainingprogress) (`DogTrainingComponent.CurrentCue` _dogtraining) (`DogTrainingComponent.GetProficiencyNormalized` _dogtraining) (`TrainingProgressComponent.IsUnlocked` _trainingprogress "Sit") (`TrainingProgressComponent.IsUnlocked` _trainingprogress "Lay") (`DogTrainingComponent.bClickWindowActive` _dogtraining)))

(fn `UserConstructionScript`)